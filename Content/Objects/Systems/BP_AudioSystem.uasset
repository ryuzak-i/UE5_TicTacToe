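; BP_AudioSystem plays the 2D music and sound effects for an X-and-O mark game.
; PlayMusic creates the passed-in sound at a lowered pitch and fades it in to the music volume.
; PlayWin stores and plays a win cue, setting its "Winner" bool parameter to distinguish ✕ from ◯, and StopWin stops it if still active.
; PlayMark fires a one-shot mark sound.
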(event Custom|PlayWin
  (params (Winner :type E_Marks%20Enum :default "NewEnumerator0"))
  (bind _returnvalue (Utilities|Name|MakeLiteralName "Winner"))
  (bind _returnvalue_2 (Audio|CreateSound2D "/Game/Resources/Audio/SFX/SC_Win.SC_Win" 1.0 1.0 0.0 0))
  (bind _output_get (Variables|Default|SetWinSound _returnvalue_2))
  (switch Utilities|FlowControl|Switch|SwitchonE_Marks Winner
    (:NewEnumerator0
      _)
    (:NewEnumerator1
      (Effects|Components|ParticleSystem|SetBoolParameter _output_get _returnvalue true))
    (:NewEnumerator2
      (Effects|Components|ParticleSystem|SetBoolParameter _output_get _returnvalue false)))
  (Audio|Components|Audio|Play _output_get 0.0))

(event Custom|PlayMark
  (Audio|PlaySound2D "/Game/Resources/Audio/SFX/SC_Mark.SC_Mark" 1.0 1.0 0.0 0 0))

(event Custom|StopWin
  (bind _winsound (Variables|Default|GetWinSound))
  (Utilities|IsValid _winsound
    (:Is%20Valid
      (switch Utilities|FlowControl|Switch|SwitchonEAudioComponentPlayState (Audio|Components|Audio|GetPlayState _winsound)
        (:Playing
          _)
        (:Paused
          _)
        (:FadingIn
          _)
        (:FadingOut
          _))
      (Audio|Components|Audio|Stop (Variables|Default|GetWinSound)))))

(event Custom|PlayMusic
  (params (NewParam :type Sound%20Base%20Object%20Reference))
  (bind _returnvalue (Audio|CreateSound2D NewParam 1.0 0.75 0.0 0))
  (bind _output_get (Variables|Default|SetMusic _returnvalue))
  (Audio|Components|Audio|FadeIn _output_get 5.0 (Variables|Default|GetMusic_Volume) 0.0 "Linear" :!class /Script/Engine.AudioComponent))

(fn ConstructionScript)