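; Game manager for an M×N, K-in-a-row tic-tac-toe match, handling turns, wins, draws and restarts.
; PrepareGame creates the UI, spawns cells into a flat indexed array with divider lines, and frames the camera over the board.
; MakeTurn scans outward from the clicked cell, using a FlipFlop to total opposite directions as one line.
; Results drive win highlighting, audio and event dispatchers, while the directional light's color follows the current turn.
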(event Custom|PrepareGame
  (Development|PrintText (Utilities|Text|FormatText "PREPARING GAME WITH M={M}, N={N}, K={K}" (Variables|Default|GetM) (Variables|Default|GetN) (Variables|Default|GetK)))
  (Utilities|FlowControl|Sequence
    (:then_0
      (bind _returnvalue (UserInterface|CreateWidget "/Game/Widgets/WBP_GameUI.WBP_GameUI_C"))
      (UserInterface|Viewport|AddtoViewport _returnvalue 0)
      (Default|CallOnGameStart)
      (Default|CallOnTurnChange))
    (:then_1
      (CallFunction|SetupCells))
    (:then_2
      (CallFunction|SetCameraTransform))
    (:then_3
      (CallFunction|HandleBackgroundColor))
    (:then_4
      (bind _returnvalue_2 (Actor|GetActorOfClass "/Game/Objects/Systems/BP_AudioSystem.BP_AudioSystem_C"))
      (Variables|Default|SetAudioSystem _returnvalue_2))))

(fn ConstructionScript)

(fn MakeTurn
  (params (ClickedCell :type BP%20Cell%20Object%20Reference))
  (bind _winner (Variables|Default|GetWinner))
  (bind _availablemoves (Variables|Default|GetAvailableMoves))
  (Variables|Default|SetClickedCell ClickedCell)
  (if (not (Variables|Default|GetIsGameEnd))
    (if (Variables|Default|GetTurn)
      (Default|AddMark (Variables|Default|GetClickedCell) "/Game/Resources/Meshes/X.X")
      (Variables|/Game/Objects/BP_Cell.BP_Cell_C|SetMarkBool (Variables|Default|GetClickedCell) true)
      (else
        (Default|AddMark (Variables|Default|GetClickedCell) "/Game/Resources/Meshes/O.O")
        (Variables|/Game/Objects/BP_Cell.BP_Cell_C|SetMarkBool (Variables|Default|GetClickedCell) false)))
    (Variables|Default|SetTurn (not (Variables|Default|GetTurn)))
    (Math|Integer|DecrementInt (Variables|Default|GetAvailableMoves)
      (:%20%20
        (CallFunction|CheckClickedCellSiblingsforWin)
        (CallFunction|HandleBackgroundColor)
        (Default|CallOnTurnChange)
        (if (Variables|Default|GetIsGameEnd)
          (Development|PrintText (Utilities|Text|FormatText "The winner is '{winner}'" (Utilities|String|EnumtoString _winner)) true true "(R=1.000000,G=1.000000,B=1.000000,A=1.000000)" 1e+01)
          (switch Utilities|FlowControl|Switch|SwitchonE_Marks _winner
            (:NewEnumerator1
              (Math|Integer|IncrementInt (Variables|Default|GetWinCountX)
                (:%20%20
                  _)))
            (:NewEnumerator2
              (Math|Integer|IncrementInt (Variables|Default|GetWinCountO)
                (:%20%20
                  _))))
          (CallFunction|ChangeWinCellsColor)
          (Default|PlayWin (Variables|Default|GetAudioSystem) (Variables|Default|GetWinner) :!label _label)
          (Default|CallOnGameEnd)
          (else
            (Development|PrintText (Utilities|Text|FormatText "Available moves = {moves}" _availablemoves))
            (if (< _availablemoves 1)
              (Development|PrintString "DRAW" true true "(R=0.937361,G=0.996018,B=1.000000,A=1.000000)" 1e+01)
              (Variables|Default|SetIsGameEnd true)
              (Default|CallOnTurnChange)
              (goto _label))))))))

(fn CheckClickedCellSiblingsforWin
  (bind _clickedcell (Variables|Default|GetClickedCell))
  (bind _clickedcell_2 (Variables|Default|GetClickedCell))
  (bind _clickedcell_3 (Variables|Default|GetClickedCell))
  (bind _wincells (Variables|Default|GetWinCells))
  (bind _clickedcell_4 (Variables|Default|GetClickedCell))
  (bind _clickedcell_5 (Variables|Default|GetClickedCell))
  (bind _clickedcell_6 (Variables|Default|GetClickedCell))
  (bind _clickedcell_7 (Variables|Default|GetClickedCell))
  (bind _clickedcell_8 (Variables|Default|GetClickedCell))
  (bind _index (Utilities|FlowControl|ForLoopwithBreak 0 (- (|GetNumEnumEntries) 1) :!label _label)
    (:LoopBody
      (bind _output_get (LocalVariables|SetDirection (Utilities|Enum|ByteToEnumE_Directions (Math|Conversions|ToByte(Integer) _index))))
      (switch Utilities|FlowControl|Switch|SwitchonE_Directions _output_get
        (:NewEnumerator0
          _)
        (:NewEnumerator1
          _)
        (:NewEnumerator2
          _)
        (:NewEnumerator3
          _)
        (:NewEnumerator4
          _)
        (:NewEnumerator5
          _)
        (:NewEnumerator6
          _)
        (:NewEnumerator7
          _))
      (Development|PrintText (Utilities|Text|FormatText "Check direction '{direction}'" (Utilities|String|EnumtoString _output_get)))
      (Utilities|FlowControl|FlipFlop
        (:A
          (Development|PrintString "CLEAR win cells and mark counter")
          (Utilities|Array|Clear _wincells)
          (Utilities|Array|Add _wincells (Variables|Default|GetClickedCell))
          (LocalVariables|SetMarkCounter 0))
        (:B
          _))
      (bind _index_2 (Utilities|FlowControl|ForLoopwithBreak 1 (- (Variables|Default|GetK) 1) :!label _label_2)
        (:LoopBody
          (LocalVariables|SetDirectionCellIndex _index_2)
          (switch Utilities|FlowControl|Switch|SwitchonE_Directions (LocalVariables|GetDirection)
            (:NewEnumerator0
              (LocalVariables|SetDirectionCheck (>= (- (Variables|/Game/Objects/BP_Cell.BP_Cell_C|GetX _clickedcell_2) (LocalVariables|GetDirectionCellIndex)) 1))
              (LocalVariables|SetDirectionCellX (- (Variables|/Game/Objects/BP_Cell.BP_Cell_C|GetX _clickedcell_2) (LocalVariables|GetDirectionCellIndex)))
              (LocalVariables|SetDirectionCellY (Variables|/Game/Objects/BP_Cell.BP_Cell_C|GetY _clickedcell_2)))
            (:NewEnumerator1
              (LocalVariables|SetDirectionCheck (<= (+ (Variables|/Game/Objects/BP_Cell.BP_Cell_C|GetX _clickedcell_3) (LocalVariables|GetDirectionCellIndex)) (Variables|Default|GetM)))
              (LocalVariables|SetDirectionCellX (+ (Variables|/Game/Objects/BP_Cell.BP_Cell_C|GetX _clickedcell_3) (LocalVariables|GetDirectionCellIndex)))
              (LocalVariables|SetDirectionCellY (Variables|/Game/Objects/BP_Cell.BP_Cell_C|GetY _clickedcell_3)))
            (:NewEnumerator2
              (LocalVariables|SetDirectionCheck (>= (- (Variables|/Game/Objects/BP_Cell.BP_Cell_C|GetY _clickedcell_4) (LocalVariables|GetDirectionCellIndex)) 1))
              (LocalVariables|SetDirectionCellX (Variables|/Game/Objects/BP_Cell.BP_Cell_C|GetX _clickedcell_4))
              (LocalVariables|SetDirectionCellY (- (Variables|/Game/Objects/BP_Cell.BP_Cell_C|GetY _clickedcell_4) (LocalVariables|GetDirectionCellIndex))))
            (:NewEnumerator3
              (LocalVariables|SetDirectionCheck (<= (+ (Variables|/Game/Objects/BP_Cell.BP_Cell_C|GetY _clickedcell_5) (LocalVariables|GetDirectionCellIndex)) (Variables|Default|GetN)))
              (LocalVariables|SetDirectionCellX (Variables|/Game/Objects/BP_Cell.BP_Cell_C|GetX _clickedcell_5))
              (LocalVariables|SetDirectionCellY (+ (Variables|/Game/Objects/BP_Cell.BP_Cell_C|GetY _clickedcell_5) (LocalVariables|GetDirectionCellIndex))))
            (:NewEnumerator4
              (LocalVariables|SetDirectionCheck (and (>= (- (Variables|/Game/Objects/BP_Cell.BP_Cell_C|GetX _clickedcell_6) (LocalVariables|GetDirectionCellIndex)) 1) (>= (- (Variables|/Game/Objects/BP_Cell.BP_Cell_C|GetY _clickedcell_6) (LocalVariables|GetDirectionCellIndex)) 1)))
              (LocalVariables|SetDirectionCellX (- (Variables|/Game/Objects/BP_Cell.BP_Cell_C|GetX _clickedcell_6) (LocalVariables|GetDirectionCellIndex)))
              (LocalVariables|SetDirectionCellY (- (Variables|/Game/Objects/BP_Cell.BP_Cell_C|GetY _clickedcell_6) (LocalVariables|GetDirectionCellIndex))))
            (:NewEnumerator5
              (LocalVariables|SetDirectionCheck (and (<= (+ (Variables|/Game/Objects/BP_Cell.BP_Cell_C|GetX _clickedcell_7) (LocalVariables|GetDirectionCellIndex)) (Variables|Default|GetM)) (<= (+ (Variables|/Game/Objects/BP_Cell.BP_Cell_C|GetY _clickedcell_7) (LocalVariables|GetDirectionCellIndex)) (Variables|Default|GetN))))
              (LocalVariables|SetDirectionCellX (+ (Variables|/Game/Objects/BP_Cell.BP_Cell_C|GetX _clickedcell_7) (LocalVariables|GetDirectionCellIndex)))
              (LocalVariables|SetDirectionCellY (+ (Variables|/Game/Objects/BP_Cell.BP_Cell_C|GetY _clickedcell_7) (LocalVariables|GetDirectionCellIndex))))
            (:NewEnumerator6
              (LocalVariables|SetDirectionCheck (and (<= (+ (Variables|/Game/Objects/BP_Cell.BP_Cell_C|GetX _clickedcell_8) (LocalVariables|GetDirectionCellIndex)) (Variables|Default|GetM)) (>= (- (Variables|/Game/Objects/BP_Cell.BP_Cell_C|GetY _clickedcell_8) (LocalVariables|GetDirectionCellIndex)) 1)))
              (LocalVariables|SetDirectionCellX (+ (Variables|/Game/Objects/BP_Cell.BP_Cell_C|GetX _clickedcell_8) (LocalVariables|GetDirectionCellIndex)))
              (LocalVariables|SetDirectionCellY (- (Variables|/Game/Objects/BP_Cell.BP_Cell_C|GetY _clickedcell_8) (LocalVariables|GetDirectionCellIndex))))
            (:NewEnumerator7
              (LocalVariables|SetDirectionCheck (and (>= (- (Variables|/Game/Objects/BP_Cell.BP_Cell_C|GetX _clickedcell) (LocalVariables|GetDirectionCellIndex)) 1) (<= (+ (Variables|/Game/Objects/BP_Cell.BP_Cell_C|GetY _clickedcell) (LocalVariables|GetDirectionCellIndex)) (Variables|Default|GetN))))
              (LocalVariables|SetDirectionCellX (- (Variables|/Game/Objects/BP_Cell.BP_Cell_C|GetX _clickedcell) (LocalVariables|GetDirectionCellIndex)))
              (LocalVariables|SetDirectionCellY (+ (Variables|/Game/Objects/BP_Cell.BP_Cell_C|GetY _clickedcell) (LocalVariables|GetDirectionCellIndex)))))
          (if (LocalVariables|GetDirectionCheck)
            (bind _result (CallFunction|GetCellbyIndex (LocalVariables|GetDirectionCellX) (LocalVariables|GetDirectionCellY)))
            (if (Variables|/Game/Objects/BP_Cell.BP_Cell_C|GetIsCellMarked _result)
              (if (== (Variables|/Game/Objects/BP_Cell.BP_Cell_C|GetMarkBool _result) (Variables|/Game/Objects/BP_Cell.BP_Cell_C|GetMarkBool (Variables|Default|GetClickedCell)))
                (Utilities|Array|Add (Variables|Default|GetWinCells) _result)
                (bind _result_2 (Math|Integer|IncrementInt (LocalVariables|GetMarkCounter))
                  (:%20%20
                    (Development|PrintText (Utilities|Text|FormatText "Found sibling cell. Win cells counter = '{counter}'. Is enough for win = {win_bool}" _result_2 (== _result_2 (- (Variables|Default|GetK) 1))))
                    (if (== _result_2 (- (Variables|Default|GetK) 1))
                      (Variables|Default|SetIsGameEnd true)
                      (Development|PrintText (Utilities|Text|FormatText "Win on '{direction}' direction" (Utilities|String|EnumtoString (LocalVariables|GetDirection))))
                      (Utilities|FlowControl|Sequence
                        (:then_0
                          (goto _label_2 Break))
                        (:then_1
                          (goto _label Break))
                        (:then_2
                          (if (Variables|/Game/Objects/BP_Cell.BP_Cell_C|GetMarkBool (Variables|Default|GetClickedCell))
                            (Variables|Default|SetWinner "NewEnumerator1")
                            (else
                              (Variables|Default|SetWinner "NewEnumerator2"))))))))
                (else
                  (goto _label_2 Break)))
              (else
                (goto _label_2 Break)))
            (else
              (goto _label_2 Break))))))
    (:Completed
      (Development|PrintString "End checking directions"))))

(fn SetupCells
  (for _index (range 1 (Variables|Default|GetM))
    (for _index_2 (range 1 (Variables|Default|GetN))
      (bind _returnvalue (Game|SpawnActorfromClass "/Game/Objects/BP_Cell.BP_Cell_C" (Math|Transform|MakeTransform "0, 0, 0") "Undefined" "MultiplyWithRoot" 0 0 0 0))
      (Variables|/Game/Objects/BP_Cell.BP_Cell_C|SetY _returnvalue _index_2)
      (Variables|/Game/Objects/BP_Cell.BP_Cell_C|SetX _returnvalue _index)
      (CallFunction|SetCellbyIndex _returnvalue)
      (CallFunction|SetCellTransform _returnvalue)
      (CallFunction|SetCellLines _returnvalue)))
  (Variables|Default|SetAvailableMoves (Utilities|Array|Length (Variables|Default|GetCells))))

(fn GetCellbyIndex
  (params (X :type Integer) (Y :type Integer))
  (bind _returnvalue (- X 1))
  (bind _cells (Variables|Default|GetCells))
  (bind _n (Variables|Default|GetN))
  (bind _returnvalue_2 (* _returnvalue _n))
  (bind _returnvalue_3 (+ _returnvalue_2 Y))
  (bind _returnvalue_4 (- _returnvalue_3 1))
  (bind _output (Utilities|Array|Get(acopy) _cells _returnvalue_4))
  (Development|PrintText (Utilities|Text|FormatText "Getting cell '{cell}' with index [{index}] (input: {x}, {y})" _output _returnvalue_4 X Y))
  (return _output))

(fn SetCellbyIndex
  (params (Cell :type BP%20Cell%20Object%20Reference))
  (bind _x (Variables|/Game/Objects/BP_Cell.BP_Cell_C|GetX Cell))
  (bind _y (Variables|/Game/Objects/BP_Cell.BP_Cell_C|GetY Cell))
  (bind _n (Variables|Default|GetN))
  (bind _returnvalue (- _x 1))
  (bind _returnvalue_2 (* _returnvalue _n))
  (bind _returnvalue_3 (+ _returnvalue_2 _y))
  (bind _returnvalue_4 (- _returnvalue_3 1))
  (Development|PrintText (Utilities|Text|FormatText "Setting cell '{cell}' with index [{index}] (input: {x}, {y})" Cell _returnvalue_4 _x _y))
  (Utilities|Array|SetArrayElem (Variables|Default|GetCells) _returnvalue_4 Cell true))

(fn SetCellTransform
  (params (Cell :type BP%20Cell%20Object%20Reference))
  (bind _boxextent (Collision|GetActorBounds Cell false false))
  (bind _x (Variables|/Game/Objects/BP_Cell.BP_Cell_C|GetX Cell))
  (bind _y (Variables|/Game/Objects/BP_Cell.BP_Cell_C|GetY Cell))
  (bind _cellsoffsetperc (Variables|Default|GetCellsOffsetPerc))
  (bind _returnvalue (/ (.x _boxextent) 1e+02))
  (bind _returnvalue_2 (* (.x _boxextent) 2.0))
  (bind _returnvalue_3 (* (.y _boxextent) 2.0))
  (bind _returnvalue_4 (/ (.y _boxextent) 1e+02))
  (bind _returnvalue_5 (* _returnvalue _cellsoffsetperc 2.0))
  (bind _returnvalue_6 (* _returnvalue_3 _x))
  (bind _returnvalue_7 (* _returnvalue_2 _y))
  (bind _returnvalue_8 (* _returnvalue_4 _cellsoffsetperc 2.0))
  (bind _returnvalue_9 (* _returnvalue_8 _x))
  (bind _returnvalue_10 (* _returnvalue_5 _y))
  (bind _returnvalue_11 (- _returnvalue_7 _returnvalue_2))
  (bind _returnvalue_12 (- _returnvalue_6 _returnvalue_3))
  (bind _returnvalue_13 (+ _returnvalue_11 _returnvalue_10))
  (bind _returnvalue_14 (+ _returnvalue_12 _returnvalue_9))
  (bind _returnvalue_15 (- _returnvalue_14 _returnvalue_8))
  (bind _returnvalue_16 (- _returnvalue_13 _returnvalue_5))
  (Development|PrintText (Utilities|Text|FormatText "For cell {x}_{y} set location {x_pos}:{y_pos}" _y _x _returnvalue_16 _returnvalue_15))
  (Transformation|SetActorTransform Cell (Math|Transform|MakeTransform (Math|Vector|MakeVector _returnvalue_16 _returnvalue_15 0.0))))

(fn SetCameraTransform
  (bind _returnvalue (Game|GetPlayerController 0))
  (bind _cells (Variables|Default|GetCells))
  (bind _cells_2 (Variables|Default|GetCells))
  (bind _cells_3 (Variables|Default|GetCells))
  (bind _returnvalue_2 (Utilities|Array|Length _cells_3))
  (bind _returnvalue_3 (Pawn|GetViewTarget _returnvalue))
  (bind _returnvalue_4 (Transformation|GetActorTransform _returnvalue_3))
  (bind _returnvalue_5 (/ _returnvalue_2 2))
  (bind _returnvalue_6 (/ _returnvalue_2 2))
  (bind _output (Utilities|Array|Get(acopy) _cells _returnvalue_5))
  (bind _output_2 (Utilities|Array|Get(acopy) _cells_2 _returnvalue_6))
  (bind _returnvalue_7 (- _returnvalue_6 1))
  (bind _returnvalue_8 (Transformation|GetActorLocation _output))
  (bind _returnvalue_9 (Transformation|GetActorLocation _output_2))
  (bind _output_3 (Utilities|Array|Get(acopy) _cells_2 _returnvalue_7))
  (bind _returnvalue_10 (Transformation|GetActorLocation _output_3))
  (bind _returnvalue_11 (- (.y _returnvalue_9) (.y _returnvalue_10)))
  (bind _returnvalue_12 (- (.x _returnvalue_10) (.x _returnvalue_9)))
  (bind _returnvalue_13 (/ _returnvalue_12 2.0))
  (bind _returnvalue_14 (/ _returnvalue_11 2.0))
  (bind _returnvalue_15 (+ (.x _returnvalue_9) _returnvalue_13))
  (bind _returnvalue_16 (+ _returnvalue_14 (.y _returnvalue_10)))
  (Development|PrintText (Utilities|Text|FormatText "Cells length = {cells_length}" _returnvalue_2))
  (bind _location_z (CallFunction|CalcCameraLocationZ))
  (if (> (Math|Integer|%(Integer) _returnvalue_2 2) 0)
    (Development|PrintText (Utilities|Text|FormatText "It's Odd. Getting pos of cell '{cell}' with index [{index}]" _output _returnvalue_5))
    (Development|PrintText (Utilities|Text|FormatText "Set camera location at X:{x_pos} Y:{y_pos} Z:{z_pos}" (.x _returnvalue_8) (.y _returnvalue_8) _location_z))
    (Transformation|SetActorTransform _returnvalue_3 (Math|Transform|MakeTransform (.location (Math|Transform|MakeTransform (Math|Vector|MakeVector (.x _returnvalue_8) (.y _returnvalue_8) _location_z))) (.rotation _returnvalue_4) (.scale _returnvalue_4)))
    (else
      (Development|PrintText (Utilities|Text|FormatText "It's Even. Calculating pos between cells '{cell_1}' [{index_1}] and '{cell_2}' [{index_2}]" _output_2 _returnvalue_6 _output_3 _returnvalue_7))
      (Development|PrintText (Utilities|Text|FormatText "Set camera location at X:{x_pos} Y:{y_pos} Z:{z_pos}" _returnvalue_15 _returnvalue_16 _location_z))
      (Transformation|SetActorTransform _returnvalue_3 (Math|Transform|MakeTransform (.location (Math|Transform|MakeTransform (Math|Vector|MakeVector _returnvalue_15 _returnvalue_16 _location_z))) (.rotation _returnvalue_4) (.scale _returnvalue_4))))))

(fn CalcCameraLocationZ
  (bind _m (Variables|Default|GetM))
  (bind _n (Variables|Default|GetN))
  (bind _cellsoffsetperc (Variables|Default|GetCellsOffsetPerc))
  (bind _returnvalue (Actor|GetActorOfClass "/Game/Objects/BP_Cell.BP_Cell_C"))
  (return (Math|Float|Max(Float) (+ (* (.x (.BoxExtent (Collision|GetActorBounds _returnvalue false false))) 2.0 _n) (* (/ (.x (.BoxExtent (Collision|GetActorBounds _returnvalue false false))) 1e+02) _cellsoffsetperc 2.0 (- _n 1))) (+ (* (.y (.BoxExtent (Collision|GetActorBounds _returnvalue false false))) 2.0 _m) (* (/ (.y (.BoxExtent (Collision|GetActorBounds _returnvalue false false))) 1e+02) _cellsoffsetperc 2.0 (- _m 1))))))

(fn ClearAllCells
  (for _array_element (Variables|Default|GetCells)
    (Default|ClearCell _array_element)))

(fn ResetGameData
  (Variables|Default|SetIsGameEnd false)
  (Variables|Default|SetWinner "NewEnumerator0")
  (Variables|Default|SetTurn true)
  (Default|CallOnTurnChange)
  (Variables|Default|SetAvailableMoves (Utilities|Array|Length (Variables|Default|GetCells)))
  (CallFunction|HandleBackgroundColor))

(fn RestartGame
  (CallFunction|ClearAllCells)
  (CallFunction|ResetGameData)
  (Default|StopWin (Variables|Default|GetAudioSystem)))

(fn HandleBackgroundColor
  (bind _returnvalue (Actor|GetActorOfClass "/Script/Engine.DirectionalLight"))
  (if (not (Variables|Default|GetIsGameEnd))
    (if (Variables|Default|GetTurn)
      (Rendering|Components|Light|SetLightColor (Variables|/Script/Engine.Light|GetLightComponent _returnvalue) "(R=1.000000,G=0.000000,B=0.333333,A=1.000000)" true)
      (else
        (Rendering|Components|Light|SetLightColor (Variables|/Script/Engine.Light|GetLightComponent _returnvalue) "(R=0.333333,G=0.000000,B=1.000000,A=1.000000)" true)))))

(fn SetCellLines
  (params (Cell :type BP%20Cell%20Object%20Reference))
  (Utilities|FlowControl|Sequence
    (:then_0
      (if (> (Variables|/Game/Objects/BP_Cell.BP_Cell_C|GetX Cell) 1)
        (bind _line_transform (CallFunction|CalcLineTransform Cell (Utilities|Map|MakeMap (Utilities|String|MakeLiteralString "Left") true)))
        (Game|SpawnActorfromClass "/Game/Objects/BP_Line.BP_Line_C" _line_transform "Undefined" "MultiplyWithRoot" 0 0)))
    (:then_1
      (if (> (Variables|/Game/Objects/BP_Cell.BP_Cell_C|GetY Cell) 1)
        (bind _line_transform_2 (CallFunction|CalcLineTransform Cell (Utilities|Map|MakeMap (Utilities|String|MakeLiteralString "Top") true)))
        (Game|SpawnActorfromClass "/Game/Objects/BP_Line.BP_Line_C" _line_transform_2 "Undefined" "MultiplyWithRoot" 0 0)))))

(fn CalcLineTransform
  (params (Cell :type BP%20Cell%20Object%20Reference) (Line_Info :type Map%20of%20Strings%20to%20Booleans))
  (bind _boxextent (Collision|GetActorBounds Cell false false))
  (bind _returnvalue (Transformation|GetActorTransform Cell))
  (bind _cellsoffsetperc (Variables|Default|GetCellsOffsetPerc))
  (bind _cellsoffsetperc_2 (Variables|Default|GetCellsOffsetPerc))
  (bind _returnvalue_2 (/ (.y (.scale _returnvalue)) 1e+02))
  (bind _returnvalue_3 (/ (.z (.scale _returnvalue)) 1e+02))
  (bind _returnvalue_4 (+ 1e+02 _cellsoffsetperc))
  (bind _returnvalue_5 (/ (.x (.scale _returnvalue)) 1e+02))
  (bind _returnvalue_6 (* _returnvalue_5 _cellsoffsetperc))
  (bind _returnvalue_7 (* _returnvalue_2 _returnvalue_4))
  (bind _returnvalue_8 (* _returnvalue_3 _cellsoffsetperc))
  (if (.Value (Utilities|Map|Find Line_Info (Utilities|String|MakeLiteralString "Left")))
    (return (Math|Transform|MakeTransform (Math|Vector|MakeVector (.x (.location _returnvalue)) (Utilities|Operators|Subtract (.y (.location _returnvalue)) (.y _boxextent) (* (/ (.y _boxextent) 1e+02) _cellsoffsetperc_2)) (.z (.location _returnvalue))) (Math|Rotator|MakeRotator (.roll (.rotation _returnvalue)) (.pitch (.rotation _returnvalue)) (+ (.yaw (.rotation _returnvalue)) 9e+01)) (Math|Vector|MakeVector _returnvalue_6 _returnvalue_7 _returnvalue_8)))
    (elif (.Value (Utilities|Map|Find Line_Info (Utilities|String|MakeLiteralString "Top")))
      (return (Math|Transform|MakeTransform (Math|Vector|MakeVector (Utilities|Operators|Subtract (.x (.location _returnvalue)) (.x _boxextent) (* (/ (.x _boxextent) 1e+02) _cellsoffsetperc_2)) (.y (.location _returnvalue)) (.z (.location _returnvalue))) (Math|Rotator|MakeRotator (.roll (.rotation _returnvalue)) (.pitch (.rotation _returnvalue)) (.yaw (.rotation _returnvalue))) (Math|Vector|MakeVector _returnvalue_6 _returnvalue_7 _returnvalue_8))))))

(fn ChangeWinCellsColor
  (for _array_element (Variables|Default|GetCells)
    (if (Variables|/Game/Objects/BP_Cell.BP_Cell_C|GetIsCellMarked _array_element)
      (if (Utilities|Array|ContainsItem (Variables|Default|GetWinCells) _array_element)
        (Rendering|Material|SetMaterial (Variables|/Game/Objects/BP_Cell.BP_Cell_C|GetMark _array_element) 0 "/Game/Resources/Materials/MI_Green.MI_Green")
        (else
          (Rendering|Material|SetMaterial (Variables|/Game/Objects/BP_Cell.BP_Cell_C|GetMark _array_element) 0 "/Game/Resources/Materials/M_Basic.M_Basic"))))))